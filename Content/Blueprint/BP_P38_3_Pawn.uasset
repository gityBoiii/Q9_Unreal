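; Player-flown P-38 plane pawn that moves along its forward vector and fires missiles.
; Tick counter-rotates the two propellers and feeds forward movement input scaled by PlaneSpeed, which the Accel axis sets.
; Roll and Pitch axes rotate the actor locally through a frame-time-scaled DeltaSpeed helper, and Fire spawns BP_Misile at the Arrow's location.
; The relative-location mover PlaneSpeedAddX is left disconnected.
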(event EventBeginPlay)

(event Collision|EventActorBeginOverlap
  (params (OtherActor :type Actor%20Object%20Reference)))

(event EventTick
  (params (DeltaSeconds :type Float%20%28single-precision%29))
  (bind _returnvalue (* DeltaSeconds 3e+03))
  (Transformation|AddRelativeRotation (Variables|Default|GetSM_P38_Propeller) (Math|Rotator|MakeRotator _returnvalue 0.0 0.0) false false)
  (Transformation|AddRelativeRotation (Variables|Default|GetSM_P38_Propeller1) (Math|Rotator|MakeRotator (* _returnvalue -1.0) 0.0 0.0) false false)
  (Pawn|Input|AddMovementInput (* (Math|Vector|GetForwardVector (Variables|Default|GetDefaultSceneRoot)) (Variables|Default|GetPlane_Speed)) 1.0 false))

(event Input|ActionEvents|InputActionFire
  (params (Key :type Key%20Structure :default "None"))
  (:Pressed
    (Game|SpawnActorfromClass "/Game/Blueprint/BP_Misile.BP_Misile_C" (Math|Transform|MakeTransform (Transformation|GetWorldLocation (Variables|Default|GetArrow)) "0, 0, 0" "1,1,1") "Undefined" 0 0)))

(event Input|AxisEvents|InputAxisRoll
  (params (AxisValue :type Float%20%28single-precision%29))
  ;[1 1 1] 속도 곱하기
  (bind _rotation (CallFunction|Delta*Speed (Variables|Default|GetRollSpeed) AxisValue))
  ;[1 1 1] 회전 결과
  (Transformation|AddActorLocalRotation (Math|Rotator|MakeRotator _rotation 0.0 0.0) false false))

(event Input|AxisEvents|InputAxisPitch
  (params (AxisValue :type Float%20%28single-precision%29))
  ;[1 1 1] 속도 곱하기
  (bind _rotation (CallFunction|Delta*Speed (Variables|Default|GetPitchSpeed) AxisValue))
  ;[1 1 1] 회전 결과
  (Transformation|AddActorLocalRotation (Math|Rotator|MakeRotator 0.0 _rotation 0.0) false false))

(event Input|AxisEvents|InputAxisAccel
  (params (AxisValue :type Float%20%28single-precision%29))
  (Variables|Default|SetPlane_Speed (* AxisValue 3.0)))

(fn ConstructionScript)

(fn PlaneSpeedAddX
  (params (DeltaLocation_X :type Float%20%28single-precision%29))
  ;[1 1 1] 비행기 속도
  (Transformation|AddRelativeLocation (Variables|Default|GetDefaultSceneRoot) (Math|Vector|MakeVector DeltaLocation_X 0.0 0.0) false false))

(fn Delta*Speed
  (params (Speed :type Float%20%28single-precision%29) (Input :type Float%20%28single-precision%29))
  (return (* (* (Utilities|Time|GetWorldDeltaSeconds) Input) Speed)))