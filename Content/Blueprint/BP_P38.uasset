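; BP_P38 is an actor, apparently a P-38 aircraft, that flies along world X at a constant speed while spinning its Left and Right components.
; Each Tick accumulates elapsed time through AddTime and prints it with a label through PrintNumber.
; That running total is the per-frame roll delta, applied in opposite directions to the two components, so their spin keeps accelerating and depends on frame rate.
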(event EventBeginPlay)

(event Collision|EventActorBeginOverlap
  (params (OtherActor :type Actor%20Object%20Reference)))

(event EventTick
  (params (DeltaSeconds :type Float%20%28single-precision%29))
  (bind _output_get (CallFunction|AddTime DeltaSeconds))
  (CallFunction|PrintNumber (Variables|Default|GetString) _output_get)
  (Transformation|AddLocalRotation (Variables|Default|GetLeft) (Math|Rotator|MakeRotator _output_get 0.0 0.0) false false)
  (Transformation|AddLocalRotation (Variables|Default|GetRight) (Math|Rotator|MakeRotator (* _output_get -1.0) 0.0 0.0) false false)
  (Transformation|AddActorWorldOffset (Math|Vector|MakeVector (* (Utilities|Time|GetWorldDeltaSeconds) 1e+02) 0.0 0.0)))

(fn ConstructionScript)

(fn AddTime
  (params (A :type Float%20%28single-precision%29))
  (bind _output_get (Variables|Default|SetSec (+ A (Variables|Default|GetSec))))
  (return _output_get))

(fn PrintNumber
  (params (A :type String) (InFloat :type Float%20%28single-precision%29))
  (Development|PrintString (Utilities|String|Append A (Utilities|String|ToString(Float) InFloat)) true true "(R=0.000000,G=0.660000,B=1.000000,A=1.000000)" 0.0))